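; Depot actor that runs a timed viewing of a depot and settles the player's bid.
; Overlapping the box slides the door open by timeline lerp and shows an observation timer widget, then a 30-second delay closes both.
; CountdownFinished removes the bid UI and deducts CurrentBid from PlayerMoney in BP_DepotPlayerState.
; The bid UI sequence that calls it and sets the one-time guard is disconnected, as is an older door-close chain.
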(event OnComponentBeginOverlap(Box)
  (params (OverlappedComponent :type Primitive%20Component%20Object%20Reference) (OtherActor :type Actor%20Object%20Reference) (OtherComp :type Primitive%20Component%20Object%20Reference) (OtherBodyIndex :type Integer) (bFromSweep :type Boolean) (SweepResult :type Hit%20Result%20Structure%20%28by%20ref%29))
  (if (not (Variables|Default|GetbIsWorkedOneTime))
    (Utilities|FlowControl|Sequence
      (:then_0
        (if (not (Variables|Default|GetbIsOpenedDoor))
          (Audio|PlaySoundatLocation "/Engine/EditorSounds/GamePreview/EjectFromPlayer.EjectFromPlayer" "0, 0, 0" "0, 0, 0" 1.0 1.0 0.0 0 0 0 0)
          (bind _openvalue (Timeline|Timeline PlayFromStart)
            (:Update
              (Transformation|SetRelativeLocation (Variables|Default|GetSM_OpenDoor) (Math|Vector|Lerp(Vector) (Variables|Default|GetClosedLoc) (Variables|Default|GetOpenLoc) _openvalue) false false)
              (Variables|Default|SetbIsOpenedDoor true)
              (Utilities|FlowControl|Delay 3e+01)
              (Variables|Default|SetbIsOpenedDoor false)
              (Widget|RemovefromParent (Variables|Default|GetObservationTimerRef))
              (Variables|Default|SetbIsOpenedTimer false)
              (Audio|PlaySoundatLocation "/Engine/EditorSounds/GamePreview/EjectFromPlayer_Cue.EjectFromPlayer_Cue" "0, 0, 0" "0, 0, 0" 1.0 1.0 0.0 0 0 0 0)
              (bind _openvalue_2 (Timeline|Timeline_1 ReverseFromEnd)
                (:Update
                  (Transformation|SetRelativeLocation (Variables|Default|GetSM_OpenDoor) (Math|Vector|Lerp(Vector) (Variables|Default|GetClosedLoc) (Variables|Default|GetOpenLoc) _openvalue_2) false false)))))))
      (:then_1
        (if (not (Variables|Default|GetbIsOpenedTimer))
          (if (Variables|Default|GetbIsOpenedDoor)
            (bind _returnvalue (UserInterface|CreateWidget "/Game/UI/Widget/WBP_ObservationTimer.WBP_ObservationTimer_C"))
            (bind _output_get (Variables|Default|SetObservationTimerRef _returnvalue))
            (UserInterface|Viewport|AddtoViewport _output_get 0)
            (Variables|Default|SetbIsOpenedTimer true)))))))

(event OnComponentEndOverlap(Box)
  (params (OverlappedComponent :type Primitive%20Component%20Object%20Reference) (OtherActor :type Actor%20Object%20Reference) (OtherComp :type Primitive%20Component%20Object%20Reference) (OtherBodyIndex :type Integer)))

(event Custom|CountdownFinished
  (bind _asbp_depot_player_state (Utilities|Casting|CastToBP_DepotPlayerState (Variables|/Script/Engine.Controller|GetPlayerState (Game|GetPlayerController 0))))
  (Widget|RemovefromParent (Variables|Default|GetBidUIRef))
  (Development|PrintString (Utilities|String|Append "KAZANAN TEKLİF " (Utilities|String|ToString(Integer) (Variables|/Game/Data/PlayerState/BP_DepotPlayerState.BP_DepotPlayerState_C|GetCurrentBid _asbp_depot_player_state))))
  (bind _asbp_depot_player_state_2 (Utilities|Casting|CastToBP_DepotPlayerState (Variables|/Script/Engine.Controller|GetPlayerState (Game|GetPlayerController 0))))
  (Variables|/Script/Engine.PlayerController|SetbShowMouseCursor (Game|GetPlayerController 0) false)
  (Development|PrintString (Utilities|String|ToString(Integer) (Variables|/Game/Data/PlayerState/BP_DepotPlayerState.BP_DepotPlayerState_C|GetCurrentBid _asbp_depot_player_state_2)))
  (bind _output_get (Variables|/Game/Data/PlayerState/BP_DepotPlayerState.BP_DepotPlayerState_C|SetPlayerMoney _asbp_depot_player_state_2 (- (Variables|/Game/Data/PlayerState/BP_DepotPlayerState.BP_DepotPlayerState_C|GetPlayerMoney _asbp_depot_player_state_2) (Variables|/Game/Data/PlayerState/BP_DepotPlayerState.BP_DepotPlayerState_C|GetCurrentBid _asbp_depot_player_state_2))))
  (Development|PrintString (Utilities|String|ToString(Integer) _output_get)))

(fn ConstructionScript)